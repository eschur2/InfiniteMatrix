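; Spawner actor that builds a chain of BP_Tunnel segments and populates them with health packs and enemies.
; On BeginPlay it destroys existing tunnels, then spawns an initial run starting at the player pawn, each following segment placed at the newest one's SpawnPoint.
; Each segment receives a reference back to the spawner, randomizes its wall, and independently rolls for a health pack and an enemy at random offsets ahead along X.
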(event EventBeginPlay
  (CallFunction|SpawnInitialTunnels))

(event Collision|EventActorBeginOverlap
  (params (OtherActor :type Actor%20Object%20Reference)))

(event EventTick
  (params (DeltaSeconds :type Float%20%28single-precision%29)))

(fn ConstructionScript)

(fn SpawnTunnel
  (params (SpawnLocation :type Vector))
  (bind _returnvalue (Game|SpawnActorfromClass "/Game/InfiniteMatrix/Blueprints/BP_Tunnel.BP_Tunnel_C" (Math|Transform|MakeTransform SpawnLocation "0, 0, 0" "1,1,1") "Undefined" 0 0))
  (bind _output_get (Variables|Default|SetNewestTunnel _returnvalue))
  (Variables|/Game/InfiniteMatrix/Blueprints/BP_Tunnel.BP_Tunnel_C|SetTunnelSpawner _output_get self)
  (Default|RandomizeWall _output_get)
  (CallFunction|SpawnHealthpackWRTLocation SpawnLocation)
  (CallFunction|SpawnEnemyWRTLocation SpawnLocation))

(fn SpawnTunnelatSpawnPoint
  (CallFunction|SpawnTunnel (Transformation|GetWorldLocation (Variables|/Game/InfiniteMatrix/Blueprints/BP_Tunnel.BP_Tunnel_C|GetSpawnPoint (Variables|Default|GetNewestTunnel)))))

(fn SpawnInitialTunnels
  (Utilities|FlowControl|Sequence
    (:then_0
      (bind _outactors (Actor|GetAllActorsOfClass "/Game/InfiniteMatrix/Blueprints/BP_Tunnel.BP_Tunnel_C"))
      (for _array_element _outactors
        (Actor|DestroyActor _array_element)))
    (:then_1
      (for _index (range 0 5)
        (Utilities|IsValid (Variables|Default|GetNewestTunnel)
          (:Is%20Valid
            (CallFunction|SpawnTunnelatSpawnPoint))
          (:Is%20Not%20Valid
            (CallFunction|SpawnTunnel (Transformation|GetActorLocation (Game|Player|GetPlayerPawn 0)))))))))

(fn SpawnHealthpackWRTLocation
  (params (Location :type Vector))
  (if (< (Math|Random|RandomFloatinRange 0.0 1.0) 0.33)
    (bind _returnvalue (Game|SpawnActorfromClass "/Game/InfiniteMatrix/Blueprints/BP_Healthpack.BP_Healthpack_C" (Math|Transform|MakeTransform (Math|Vector|MakeVector (+ (.x Location) (Math|Random|RandomFloatinRange 7e+02 1.7e+03)) (+ (.y Location) (Math|Random|RandomFloatinRange -3e+02 3e+02)) (+ (.z Location) (Math|Random|RandomFloatinRange -3e+02 3e+02))) "0, 0, 0" "1,1,1") "Undefined" 0 0))
    (Variables|Default|SetNewestHealthpack _returnvalue)))

(fn SpawnEnemyWRTLocation
  (params (Location :type Vector))
  (if (< (Math|Random|RandomFloatinRange 0.0 1.0) 0.33)
    (bind _returnvalue (Game|SpawnActorfromClass "/Game/InfiniteMatrix/Blueprints/BP_Enemy.BP_Enemy_C" (Math|Transform|MakeTransform (Math|Vector|MakeVector (+ (.x Location) (Math|Random|RandomFloatinRange 7e+02 1.7e+03)) (+ (.y Location) (Math|Random|RandomFloatinRange -1.5e+02 1.5e+02)) (+ (.z Location) (Math|Random|RandomFloatinRange -1.5e+02 1.5e+02))) "0, 0, 0" "1,1,1") "Undefined" 0 0))
    (Variables|Default|SetNewestEnemy _returnvalue)))